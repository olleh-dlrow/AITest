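; AI-controlled character Blueprint with an attached assault rifle that takes point damage and feeds combat state to its blackboard.
; Perception is used only to spot the player, setting the target and raising aim weight.
; A per-tick visibility trace to the player sets HasSight for whether a shot can land.
; Point damage lowers clamped health, spawns blood, flags Injured and targets the damage causer.
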(event `self.ReceivePointDamage`
  (params (Damage :type "Float (single-precision)") (DamageType :type "DamageType Object Reference") (HitLocation :type "Vector Structure") (HitNormal :type "Vector Structure") (HitComponent :type "PrimitiveComponent Object Reference") (BoneName :type Name) (ShotFromDirection :type "Vector Structure") (InstigatedBy :type "Controller Object Reference") (DamageCauser :type "Actor Object Reference") (HitInfo :type "HitResult Structure (by ref)"))
  ;[1 1 1] GetDamage
  (set `self.Health` (`KismetMathLibrary.FClamp` (- (`self.Health`) Damage) 0.0 100.0))
  (`GameplayStatics.SpawnEmitterAtLocation` "/Game/WeaponEffects/BloodImpact/P_blood_splash_02.P_blood_splash_02" HitLocation)
  (`self.UpdateInjuredKey` true)
  (`self.UpdateTargetKey` DamageCauser))

(event `self.ReceiveTick`
  (params (DeltaSeconds :type "Float (single-precision)"))
  ;[1 1 1] Tick
  (`self.CheckTraceHit`))

(event `UpdateSightKey`
  (params (HasSight :type Boolean))
  ;[1 1 1] UpdateSightKey
  (`BlackboardComponent.SetValueAsBool` (`AIBlueprintHelperLibrary.GetBlackboard` null) "HasSight" HasSight))

(event `self.AIPerception.OnTargetPerceptionUpdated`
  (params (Actor :type "Actor Object Reference") (Stimulus :type "AIStimulus Structure"))
  ;[1 1 1] 视野检测只用于发现玩家
  (set `self.TargetActor` Actor)
  (if (`self.ActorHasTag` Actor "Player")
    (if (`.bSuccessfullySensed` (break `AIStimulus` Stimulus))
      (`self.UpdateTargetKey` (`self.TargetActor`))
      (set `self.AimWeight` 1.0))))

(event `UpdateTargetKey`
  (params (Actor :type "Object Object Reference"))
  ;[1 1 1] UpdateTargetKey
  (`BlackboardComponent.SetValueAsObject` (`AIBlueprintHelperLibrary.GetBlackboard` null) "TargetActor" Actor))

(event `CheckTraceHit`
  (bind _returnvalue (`GameplayStatics.GetPlayerCharacter` 0))
  ;[1 1 1] 是否能够射击命中玩家
  (`/Engine/EditorBlueprintResources/StandardMacros.IsValid` _returnvalue
    (:`Is Valid`
      (bind _outhit (`KismetSystemLibrary.LineTraceSingle` (`self.K2_GetActorLocation`) (`self.K2_GetActorLocation` _returnvalue) "TraceTypeQuery1" false (`|MakeArray` self :!type "Actor Object Reference")))
      (if (`self.ActorHasTag` (`.HitActor` (`GameplayStatics.BreakHitResult` _outhit)) "Player")
        (`self.UpdateSightKey` true)
        (else
          (`self.UpdateSightKey` false))))))

(event `UpdateInjuredKey`
  (params (Injured :type Boolean))
  ;[1 1 1] UpdateInjuredKey
  (`BlackboardComponent.SetValueAsBool` (`AIBlueprintHelperLibrary.GetBlackboard` null) "Injured" Injured))

(fn `UserConstructionScript`
  (`SceneComponent.K2_AttachToComponent` (`self.SK_AssaultRifle`) (`self.Mesh`) "GunSocket" "KeepRelative" "KeepRelative" "KeepRelative" true))